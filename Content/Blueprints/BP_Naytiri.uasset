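; BP_Naytiri is a multiplayer player character with sword or magic combat, dash, grappling hook and death/respawn.
; On BeginPlay it polls PlayerState, sends customization settings to the server, applies cosmetics and adds HUD widgets.
; Server-to-multicast event pairs drive animation states, attack radius, magic effects and grappling, with weapon type selecting attacks.
; Grappling applies steerable force each tick; death triggers ragdoll and a death screen, and restarting respawns at a random PlayerStart.
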(event `self.ReceiveTick`
  (params (DeltaSeconds :type "Float (single-precision)"))
  (bind _index (`self.Index`))
  ;[0.2812 0.003141 0] Class Debug Shower
  (`|ExecutionSequence`
    (:`then_0`
      (`TextRenderComponent.K2_SetText` _index (`KismetTextLibrary.Conv_DoubleToText` (`self.Health`) "HalfToEven"))
      (`SceneComponent.K2_SetWorldRotation` _index (`KismetMathLibrary.FindLookAtRotation` (`SceneComponent.K2_GetComponentLocation` _index) (`SceneComponent.K2_GetComponentLocation` (`self.mCamera`))) false false))
    (:`then_1`
      (`self.GrappleTick`))))

(event `DeathScreen`
  ;[0 0 0] Death Screen
  (`/Engine/EditorBlueprintResources/StandardMacros.IsValid` (`self.Death_W`)
    (:`Is Valid`
      _)
    (:`Is Not Valid`
      (bind _returnvalue (`|CreateWidget` "/Game/Final/Widget/Death_W.Death_W_C"))
      (bind _output_get (set `self.Death_W` _returnvalue))))
  (`UserWidget.AddToViewport` _output_get 0)
  (set `PlayerController.bShowMouseCursor` true (`GameplayStatics.GetPlayerController` 0)))

(event `self.ReceiveBeginPlay`
  ;[0.2834 0.3136 1] EventBeginPlay
  (`|ExecutionSequence`
    (:`then_0`
      (bind _asnaytiri_anim_bp_base_character (cast `/Game/Final/Animations/Naytiri_AnimBP_BaseCharacter` (`SkeletalMeshComponent.GetAnimInstance` (`self.Mesh`))))
      (bind _output_get (set `self.Naytiri_Animation` _asnaytiri_anim_bp_base_character))
      (`COACharAnimInstance.ChangeAnimState` _output_get "CAS_UNKNOWN")
      ;[1 0.8977 0.05415] Structure Implementasyonu (Player Sends its settings to Server)
      (bind _playerstate (`self.PlayerState` :!label _label)
        (:`then`
          (if (`self.IsLocallyControlled`)
            (`self.SendPlayerSettingsServer` (`/Game/Blueprints/BP_COAGameInstance.PlayerSettings` (cast `/Game/Blueprints/BP_COAGameInstance` (`GameplayStatics.GetGameInstance`) :!pure true))))
          (bind _asbp_coaplayer_state (cast `/Game/Blueprints/BP_COAPlayerState` _playerstate :!label _label_2))
          (if (`/Game/Blueprints/BP_COAPlayerState.SettingsReady` _asbp_coaplayer_state)
            (bind (_settings_displayname _settings_costumecolor _settings_weapontype _settings_hattype _settings_shoetype) (break `/Game/Blueprints/S_PlayerSettings` (`/Game/Blueprints/BP_COAPlayerState.Settings` _asbp_coaplayer_state)))
            (`MeshComponent.SetVectorParameterValueOnMaterials` (`self.Mesh`) "BodyColor" (`KismetMathLibrary.Conv_LinearColorToVector` _settings_costumecolor))
            (`self.PlayerName Multicast` _settings_displayname)
            (`self.ChangeWeapon Multicast` _settings_weapontype)
            (`self.ChangeHat Multicast` _settings_hattype)
            (`self.ChangeShoe Multicast` _settings_shoetype)
            (else
              (`KismetSystemLibrary.Delay` 0.2)
              (goto _label_2))))
        (:`else`
          (`KismetSystemLibrary.Delay` 0.2)
          (goto _label))))
    (:`then_1`
      (bind _returnvalue (`GameplayStatics.GetCurrentLevelName` true))
      (if (or (`KismetStringLibrary.NotEqual_StrStr` _returnvalue "MainMenu") (`KismetStringLibrary.NotEqual_StrStr` _returnvalue "CharacterCustomization") (`KismetStringLibrary.NotEqual_StrStr` _returnvalue "Char"))
        (`/Engine/EditorBlueprintResources/StandardMacros.IsValid` (`self.Crosshair_W`)
          (:`Is Valid`
            _)
          (:`Is Not Valid`
            (bind _returnvalue_2 (`|CreateWidget` "/Game/Final/Widget/Crosshair_W.Crosshair_W_C"))
            (bind _output_get_2 (set `self.Crosshair_W` _returnvalue_2))))
        (`UserWidget.AddToViewport` _output_get_2 0)
        (`/Engine/EditorBlueprintResources/StandardMacros.IsValid` (`self.GUI_W`)
          (:`Is Valid`
            _)
          (:`Is Not Valid`
            (bind _returnvalue_3 (`|CreateWidget` "/Game/Final/Widget/GUI_W.GUI_W_C"))
            (bind _output_get_3 (set `self.GUI_W` _returnvalue_3))))
        (`UserWidget.AddToViewport` _output_get_3 0)))))

(event `InputAction|Attack`
  (params (Key :type "Key Structure"))
  (:`Pressed`
    (`self.Idle?`
      (:`IdleYes`
        (bind _settings (`self.StateMacro`))
        (if (`|EnumEquality` (`.WeaponType_9_909028214361E467878D2E935A1A49CC` (break `/Game/Blueprints/S_PlayerSettings` _settings)) "NewEnumerator2")
          ;[1 1 1] Magic İse
          (`self.ChangeAttackRadius&StateServer` 0.0)
          (`self.ChangeAnimStateServer` "CAS_CAST")
          (`self.Client`)
          (else
            ;[1 1 1] Normal İse
            (`self.ChangeAttackRadius&StateServer` 25.0 150.0)
            (`self.ChangeAnimStateServer` "CAS_ATTACK")))))))

(event `FireBall`
  ;[1 0.339 0.2191] FireBall
  (`KismetSystemLibrary.Delay` 0.3)
  (`|SpawnActorFromClass` "/Game/Blueprints/A2/FireBall.FireBall_C" (`KismetMathLibrary.MakeTransform` (`SceneComponent.K2_GetComponentLocation` (`self.FireBallS`)) (`self.K2_GetActorRotation`) (0.5 0.5 0.5)) "AlwaysSpawn" "OverrideRootScale" null (`self.ChangeMagicType`) null)
  (set `self.FireBallCooldown` true)
  (`KismetSystemLibrary.Delay` 2.0)
  (set `self.FireBallCooldown` false))

(event `ChangeShoe Multicast`
  (params (`Shoe Type` :type "/Game/Blueprints/E_CostumeShoeType Enum" :default "NewEnumerator0"))
  ;[0 0 0] ChangeShoe Multicast
  (switch `/Game/Blueprints/E_CostumeShoeType` `Shoe Type`
    (:`NewEnumerator0`
      (`SceneComponent.SetVisibility` (`self.Shoe1 - R`) false false)
      (`SceneComponent.SetVisibility` (`self.Shoe1 - L`) false false))
    (:`NewEnumerator1`
      (`SceneComponent.SetVisibility` (`self.Shoe1 - R`) true false)
      (`SceneComponent.SetVisibility` (`self.Shoe1 - L`) true false)
      (`StaticMeshComponent.SetStaticMesh` (`self.Shoe1 - R`) "/Game/Final/Models/Shoe1/Shoe1.Shoe1")
      (`StaticMeshComponent.SetStaticMesh` (`self.Shoe1 - L`) "/Game/Final/Models/Shoe1/Shoe1.Shoe1"))
    (:`NewEnumerator2`
      (`SceneComponent.SetVisibility` (`self.Shoe1 - R`) true false)
      (`SceneComponent.SetVisibility` (`self.Shoe1 - L`) true false)
      (`StaticMeshComponent.SetStaticMesh` (`self.Shoe1 - R`) "/Game/Final/Models/Shoe2/Shoe2.Shoe2")
      (`StaticMeshComponent.SetStaticMesh` (`self.Shoe1 - L`) "/Game/Final/Models/Shoe2/Shoe2.Shoe2"))
    (:`NewEnumerator3`
      (`SceneComponent.SetVisibility` (`self.Shoe1 - R`) true false)
      (`SceneComponent.SetVisibility` (`self.Shoe1 - L`) true false)
      (`StaticMeshComponent.SetStaticMesh` (`self.Shoe1 - R`) "/Game/Final/Models/Slipper/Slipper.Slipper")
      (`StaticMeshComponent.SetStaticMesh` (`self.Shoe1 - L`) "/Game/Final/Models/Slipper/Slipper.Slipper"))))

(event `ChangeHat Multicast`
  (params (`Hat Type` :type "/Game/Blueprints/E_CostumeHatType Enum" :default "NewEnumerator0"))
  ;[0 0 0] ChangeHat Multicast
  (switch `/Game/Blueprints/E_CostumeHatType` `Hat Type`
    (:`NewEnumerator0`
      (`SceneComponent.SetVisibility` (`self.Hat - Samurai`) false false)
      (`SceneComponent.SetVisibility` (`self.Hat - Wizard`) false false)
      (`SceneComponent.SetVisibility` (`self.Hat - Cowboy`) false false))
    (:`NewEnumerator1`
      (`SceneComponent.SetVisibility` (`self.Hat - Samurai`) false false)
      (`SceneComponent.SetVisibility` (`self.Hat - Wizard`) false false)
      (`SceneComponent.SetVisibility` (`self.Hat - Cowboy`) false false)
      (`SceneComponent.SetVisibility` (`self.Hat - Cowboy`) true false))
    (:`NewEnumerator2`
      (`SceneComponent.SetVisibility` (`self.Hat - Samurai`) false false)
      (`SceneComponent.SetVisibility` (`self.Hat - Wizard`) false false)
      (`SceneComponent.SetVisibility` (`self.Hat - Cowboy`) false false)
      (`SceneComponent.SetVisibility` (`self.Hat - Wizard`) true false))
    (:`NewEnumerator3`
      (`SceneComponent.SetVisibility` (`self.Hat - Samurai`) false false)
      (`SceneComponent.SetVisibility` (`self.Hat - Wizard`) false false)
      (`SceneComponent.SetVisibility` (`self.Hat - Cowboy`) false false)
      (`SceneComponent.SetVisibility` (`self.Hat - Samurai`) true false))))

(event `PlayerName Multicast`
  (params (InString :type String))
  ;[0 0 0] Player name Multicast
  (`TextRenderComponent.K2_SetText` (`self.PlayerName`) (`KismetTextLibrary.Conv_StringToText` InString)))

(event `ChangeWeapon Multicast`
  (params (WeaponType :type "/Game/Blueprints/E_WeaponType Enum" :default "NewEnumerator0"))
  (bind _sword (`self.Sword`))
  ;[0 0 0] Change Weapon Multicast
  (switch `/Game/Blueprints/E_WeaponType` WeaponType
    (:`NewEnumerator0`
      (`SceneComponent.SetHiddenInGame` _sword true false)
      (`SceneComponent.SetHiddenInGame` (`self.Niagara_HandLeft`) true false)
      (`SceneComponent.SetHiddenInGame` (`self.Niagara_HandRight`) true false))
    (:`NewEnumerator1`
      (`SceneComponent.SetHiddenInGame` _sword false false)
      (`SceneComponent.SetHiddenInGame` (`self.Niagara_HandLeft`) true false)
      (`SceneComponent.SetHiddenInGame` (`self.Niagara_HandRight`) true false))
    (:`NewEnumerator2`
      (`SceneComponent.SetHiddenInGame` _sword true false)
      (`SceneComponent.SetHiddenInGame` (`self.Niagara_HandRight`) false false)
      (`SceneComponent.SetHiddenInGame` (`self.Niagara_HandLeft`) false false))))

(event `Client`
  ;[1 1 1] Büyü Yaparken Dönmek İçin
  (set `self.bUseControllerRotationYaw` true)
  (`self.Server`)
  (`KismetSystemLibrary.Delay` 1.0)
  (set `self.bUseControllerRotationYaw` false))

(event `Key|Y`
  (params (Key :type "Key Structure"))
  (bind (_settings_displayname _settings_costumecolor _settings_weapontype) (break `/Game/Blueprints/S_PlayerSettings` (`/Game/Blueprints/BP_COAPlayerState.Settings` (cast `/Game/Blueprints/BP_COAPlayerState` (`self.PlayerState`) :!pure true))))
  (:`Pressed`
    (`KismetSystemLibrary.PrintString` (`|GetEnumeratorNameAsString` _settings_weapontype))))

(event `ChangeAttackRadius&StateServer`
  (params (AttackDamage :type "Float (double-precision)") (InSphereRadius :type "Float (double-precision)") (SlowAttack :type Boolean) (MagicSlowAttack :type Boolean))
  ;[0 0 0] Change Attack Radius Server / Multi
  (`self.ChangeAttackRadius&StateMulti` AttackDamage InSphereRadius SlowAttack MagicSlowAttack))

(event `Server`
  ;[1 1 1] Büyü Yaparken Dönmek İçin
  (set `self.bUseControllerRotationYaw` true)
  (`KismetSystemLibrary.Delay` 1.0)
  (set `self.bUseControllerRotationYaw` false))

(event `SmallShot`
  (params (`Spawn Transform Location` :type "Vector Structure") (`Spawn Transform Rotation` :type "Rotator Structure"))
  ;[1 1 1] Small Shot Casting
  (`|SpawnActorFromClass` "/Game/Blueprints/A2/SmallShot.SmallShot_C" (`KismetMathLibrary.MakeTransform` `Spawn Transform Location` `Spawn Transform Rotation` (0.2 0.2 0.2)) "AlwaysSpawn" "OverrideRootScale" null self null)
  (`KismetSystemLibrary.Delay` 1.0)
  (set `self.bUseControllerRotationYaw` false))

(event `ChangeAttackRadius&StateMulti`
  (params (AttackDamage :type "Float (double-precision)") (InSphereRadius :type "Float (double-precision)") (SlowAttack :type Boolean) (MagicSlowAttack :type Boolean))
  ;[0 0 0] Change Attack Radius Server / Multi
  (`self.Radius/Damage` AttackDamage InSphereRadius)
  (set `self.SlowAttack` SlowAttack)
  (set `self.MagicSlowAttack` MagicSlowAttack))

(event `Key|C`
  (params (Key :type "Key Structure"))
  ;[1 1 1] Special Attack
  (:`Pressed`
    (`self.Idle?`
      (:`IdleYes`
        (`self.Special Attack`)))))

(event `SpecialAttackServer`
  ;[1 1 1] Special Attack
  (`|SpawnActorFromClass` "/Game/Blueprints/A2/IceWave.IceWave_C" (`KismetMathLibrary.MakeTransform` (`self.K2_GetActorLocation`)) "AlwaysSpawn" "OverrideRootScale" null self null))

(event `ChangeDisplayName Multicast`
  (params (`Display Name` :type String))
  ;[0 0 0] ChangeDisplayName Multicast
  (`TextRenderComponent.K2_SetText` (`self.PlayerName`) (`KismetTextLibrary.Conv_StringToText` `Display Name`)))

(event `ChangeAnimStateServer`
  (params (NewState :type "ECharAnimState Enum" :default "CAS_UNKNOWN"))
  ;[0 0 0] Change Anim State Server / Multi
  (`self.ChangeAnimStateMulti` NewState))

(event `Special Attack`
  ;[1 1 1] Special Attack
  (if (not (`self.SpecialAttackCD`))
    (set `self.SpecialAttackCD` true)
    (`self.ChangeAnimStateServer` "CAS_SPECIAL")
    (`KismetSystemLibrary.Delay` 15.0)
    (set `self.SpecialAttackCD` false)))

(event `SmallShotLocClient`
  (bind _returnvalue (`SceneComponent.K2_GetComponentRotation` (`self.mCamera`)))
  (bind (_returnvalue_location _returnvalue_rotation) (`KismetMathLibrary.BreakTransform` (`KismetMathLibrary.MakeTransform` (+ (`SceneComponent.K2_GetComponentLocation` (`self.ShotBall`)) (`KismetMathLibrary.Conv_RotatorToVector` _returnvalue)) _returnvalue (0.2 0.2 0.2))))
  ;[1 1 1] Small Shot Casting
  (`self.SmallShot` _returnvalue_location _returnvalue_rotation))

(event `ChangeAnimStateMulti`
  (params (NewState :type "ECharAnimState Enum" :default "CAS_UNKNOWN"))
  ;[0 0 0] Change Anim State Server / Multi
  (`self.ChangeAnimState` NewState))

(event `NiagaraSpecialServer`
  (params (Target :type "NiagaraComponent Object Reference") (InAsset :type "NiagaraSystem Object Reference"))
  ;[1 1 1] Special Attack
  (`self.NiagaraSpecialMulticast` Target InAsset))

(event `NiagaraSpecialMulticast`
  (params (Target :type "NiagaraComponent Object Reference") (InAsset :type "NiagaraSystem Object Reference"))
  ;[1 1 1] Special Attack
  (`NiagaraComponent.SetAsset` Target InAsset true)
  (`KismetSystemLibrary.Delay` 4.0)
  (`NiagaraComponent.SetAsset` Target "/Game/MagicTrails/FX/NS_Body_Air.NS_Body_Air" true))

(event `Key|LeftAlt`
  (params (Key :type "Key Structure"))
  (bind _returnvalue (`GameplayStatics.GetPlayerController` 0))
  (bind _returnvalue_2 (or (`PlayerController.IsInputKeyDown` _returnvalue "W") (`PlayerController.IsInputKeyDown` _returnvalue "A") (`PlayerController.IsInputKeyDown` _returnvalue "S") (`PlayerController.IsInputKeyDown` _returnvalue "D")))
  ;[0.3008 0.9602 1] Dash Input
  (:`Pressed`
    (if _returnvalue_2
      (`self.Dash`)))
  (:`Released`
    (if _returnvalue_2
      _)))

(event `Dash`
  (bind _stamina (`self.Stamina`))
  ;[0.3735 1 0.2551] Dash
  (if (and (> _stamina 20.0) (not (`self.bStaminaDrained`)))
    (`/Engine/EditorBlueprintResources/StandardMacros.DoOnce` false :!label _label_3
      (:`Completed`
        (set `self.Stamina` (- _stamina 20.0))
        (`self.LaunchCharacter` (0.0 0.0 200.0))
        (`KismetSystemLibrary.Delay` 0.1)
        (`self.LaunchCharacter` (* (`KismetMathLibrary.GetForwardVector` (`self.K2_GetActorRotation`)) (`self.DashMeter`)))
        (`KismetSystemLibrary.Delay` 1.0)
        (goto _label_3 :!via `Reset`)))))

(event `SendPlayerSettingsServer`
  (params (Settings :type "/Game/Blueprints/S_PlayerSettings Structure"))
  ;[1 0.3811 0.8593] Server Validates and Replicates Back!
  (bind _playerstate (`self.PlayerState`)
    (:`then`
      (bind _asbp_coaplayer_state (cast `/Game/Blueprints/BP_COAPlayerState` _playerstate))
      (set `/Game/Blueprints/BP_COAPlayerState.Settings` Settings _asbp_coaplayer_state))
    (:`else`)))

(event `PlayAnimMontageMultiCast`
  ;[1 1 1] OOF
  (`self.PlayAnimMontage` self "/Game/MagicalAnimSet/Animations/attack/10_buff/İceWave.İceWave" 1.0 "None"))

(event `InputAction|Grapple`
  (params (Key :type "Key Structure"))
  (bind _returnvalue (`GameplayStatics.GetPlayerCameraManager` 0))
  (bind _returnvalue_2 (`PlayerCameraManager.GetCameraLocation` _returnvalue))
  ;[0.0648 0.3325 0.05951] Input Grapple
  (:`Pressed`
    (bind (_outhit _returnvalue_3) (`KismetSystemLibrary.LineTraceSingleForObjects` _returnvalue_2 (+ _returnvalue_2 (* (`self.GetActorForwardVector` _returnvalue) 10000.0)) (`|MakeArray` "ObjectTypeQuery9" :!type "EObjectTypeQuery Enum")))
    (if _returnvalue_3
      (`self.GrapnelServer` (`.ImpactPoint` (`GameplayStatics.BreakHitResult` _outhit)))))
  (:`Released`
    (`self.GrapnelReleaseServer`)))

(event `GrapnelServer`
  (params (GrapplePointLocation :type "Vector Structure"))
  ;[0.0648 0.3325 0.05951] Input Grapple
  (`self.GrapnelMulticast` GrapplePointLocation))

(event `Ragdoll`
  ;[0.3813 0.536 1] Ragdoll when slained
  (`PrimitiveComponent.SetSimulatePhysics` (`self.Mesh`) true)
  (`CharacterMovementComponent.DisableMovement` (`self.CharacterMovement`))
  (`PrimitiveComponent.SetCollisionProfileName` (`self.Mesh`) "Ragdoll" true))

(event `GrapnelMulticast`
  (params (GrapplePointLocation :type "Vector Structure"))
  ;[0.0648 0.3325 0.05951] Input Grapple
  (set `self.GrapplePointLocation` GrapplePointLocation)
  (set `self.isGrappling?` true)
  (`CharacterMovementComponent.SetMovementMode` (`self.CharacterMovement`) "MOVE_Falling" 0)
  (`SceneComponent.SetVisibility` (`self.GrapplingCable`) true false))

(event `InputAction|SecondaryAttack`
  (params (Key :type "Key Structure"))
  ;[0.5174 0.7373 1] Secondary Attack
  (:`Pressed`
    (`self.Idle?`
      (:`IdleYes`
        (bind _settings (`self.StateMacro`))
        (if (`|EnumEquality` (`.WeaponType_9_909028214361E467878D2E935A1A49CC` (break `/Game/Blueprints/S_PlayerSettings` _settings)) "NewEnumerator2")
          (if (not (`self.FireBallCooldown`))
            ;;[1 1 1] Magic ise slow attack radius off
            (`self.ChangeAttackRadius&StateServer` 0.0 0.0 false true)
            (`self.FireBall`)
            (`self.ChangeAnimStateServer` "CAS_CAST"))
          (else
            (`self.ChangeAttackRadius&StateServer` 35.0 250.0 true)
            (`self.ChangeAnimStateServer` "CAS_ATTACK"))))))
  (:`Released`
    (bind _settings_2 (`self.StateMacro`))
    (if (`|EnumEquality` (`.WeaponType_9_909028214361E467878D2E935A1A49CC` (break `/Game/Blueprints/S_PlayerSettings` _settings_2)) "NewEnumerator2")
      (`KismetSystemLibrary.Delay` 1.0)
      (set `self.MagicSlowAttack` false)
      (else
        (`KismetSystemLibrary.Delay` 1.0)
        (set `self.SlowAttack` false)))))

(event `NiagaraMulticast`
  (params (Magic :type "/Game/Blueprints/MagicTrails Enum" :default "NewEnumerator0"))
  (bind _niagara_handright (`self.Niagara_HandRight`))
  ;[1 0.8264 0.4463] Niagara Effects/ Change Magic Type
  (switch `/Game/Blueprints/MagicTrails` Magic
    (:`NewEnumerator0`
      (`NiagaraComponent.SetAsset` (`self.Niagara_HandLeft`) "/Game/MagicTrails/FX/NS_Hands_Dark.NS_Hands_Dark" true)
      (`NiagaraComponent.SetAsset` _niagara_handright "/Game/MagicTrails/FX/NS_Hands_Dark.NS_Hands_Dark" true))
    (:`NewEnumerator1`
      (`NiagaraComponent.SetAsset` _niagara_handright "/Game/MagicTrails/FX/NS_Hands_Air.NS_Hands_Air" true)
      (`NiagaraComponent.SetAsset` (`self.Niagara_HandLeft`) "/Game/MagicTrails/FX/NS_Hands_Air.NS_Hands_Air" true))
    (:`NewEnumerator2`
      (`NiagaraComponent.SetAsset` _niagara_handright "/Game/MagicTrails/FX/NS_Hands_Electric.NS_Hands_Electric" true)
      (`NiagaraComponent.SetAsset` (`self.Niagara_HandLeft`) "/Game/MagicTrails/FX/NS_Hands_Electric.NS_Hands_Electric" true))
    (:`NewEnumerator4`
      (`NiagaraComponent.SetAsset` (`self.Niagara_HandRight`) "/Game/MagicTrails/FX/NS_Hands_Fire.NS_Hands_Fire" true)
      (`NiagaraComponent.SetAsset` (`self.Niagara_HandLeft`) "/Game/MagicTrails/FX/NS_Hands_Fire.NS_Hands_Fire" true))
    (:`NewEnumerator3`
      (`NiagaraComponent.SetAsset` (`self.Niagara_HandLeft`) "/Game/MagicTrails/FX/NS_Hands_Poison.NS_Hands_Poison" true)
      (`NiagaraComponent.SetAsset` (`self.Niagara_HandRight`) "/Game/MagicTrails/FX/NS_Hands_Poison.NS_Hands_Poison" true))))

(event `GrapnelReleaseServer`
  ;[0.0648 0.3325 0.05951] Input Grapple
  (`self.GrapnelReleaseMulti`))

(event `NiagaraServer`
  (params (Magic :type "/Game/Blueprints/MagicTrails Enum" :default "NewEnumerator0"))
  ;[1 0.8264 0.4463] Niagara Effects/ Change Magic Type
  (bind _output_get (set `self.ChangeMagicType` Magic))
  (`self.NiagaraMulticast` _output_get))

(event `GrapnelReleaseMulti`
  ;[0.0648 0.3325 0.05951] Input Grapple
  (set `self.isGrappling?` false)
  (`CharacterMovementComponent.SetMovementMode` (`self.CharacterMovement`) "MOVE_Falling" 0)
  (`SceneComponent.SetVisibility` (`self.GrapplingCable`) false false))

(event `Key|T`
  (params (Key :type "Key Structure"))
  ;[1 0.8264 0.4463] Niagara Effects/ Change Magic Type
  (:`Pressed`
    (bind _output_get (set `self.ChangeMagicType` (cast `/Game/Blueprints/MagicTrails` (`KismetMathLibrary.Conv_IntToByte` (`KismetMathLibrary.RandomIntegerInRange` 0 5)))))
    (`self.NiagaraServer` _output_get)))

(event `GrappleTick`
  ;[0.0648 0.3325 0.05951] Grapple Tick
  (if (`self.isGrappling?`)
    (`CharacterMovementComponent.AddForce` (`self.CharacterMovement`) (* (`KismetMathLibrary.Normal` (+ (`KismetMathLibrary.GetDirectionUnitVector` (`self.K2_GetActorLocation`) (`self.GrapplePointLocation`)) (* (* (`self.GetActorRightVector`) (`self.GetInputAxisValue`)) 0.5))) 300000.0))
    (set `CableComponent.EndLocation` (`KismetMathLibrary.InverseTransformLocation` (`self.GetTransform`) (`self.GrapplePointLocation`)) (`self.GrapplingCable`))
    (if (<= (`KismetMathLibrary.Vector_Distance` (`self.GrapplePointLocation`) (`self.K2_GetActorLocation`)) 100.0)
      (set `self.isGrappling?` false)
      (`MovementComponent.StopMovementImmediately` (`self.CharacterMovement`)))))

(event `self.ReceiveDestroyed`
  ;[1 0.4682 0.4582] Respawn
  (bind _asgameplay_game_mode (cast `/Game/Final/GameMode/GameplayGameMode` (`GameplayStatics.GetGameMode`)))
  (`/Game/Final/GameMode/GameplayGameMode.PlayerDied` _asgameplay_game_mode self))

(event `RestartPlayer Server`
  ;[0 0 0] RestartPlayer Server
  (`self.Call Restart Player`))

(event `RespawnChar`
  ;[1 0.07208 0] Respawn Mechanic
  (bind _asbp_gameplay_controller (cast `/Game/Final/GameMode/BP_GameplayController` (`GameplayStatics.GetPlayerController` 0)))
  (bind _returnvalue (`GameplayStatics.GetActorOfClass` "/Script/Engine.PlayerStart"))
  (`/Game/Final/GameMode/BP_GameplayController.RespawnPawn` _asbp_gameplay_controller (`self.GetTransform` _returnvalue) (`Controller.K2_GetPawn` _asbp_gameplay_controller))
  (`Controller.UnPossess` _asbp_gameplay_controller))

(fn `Call Restart Player`
  (locals (ControllerRef :type "Controller Object Reference"))
  (set `local.ControllerRef` (`self.GetController`))
  (`self.K2_DestroyActor`)
  (bind _outactors (`GameplayStatics.GetAllActorsOfClass` "/Script/Engine.PlayerStart"))
  (bind _returnvalue (`|SpawnActorFromClass` "BP_Naytiri_C" (`self.GetTransform` (`|GetArrayItem` _outactors (`KismetMathLibrary.RandomInteger` (`KismetArrayLibrary.Array_Length` _outactors)))) "Undefined" "OverrideRootScale" null (struct) null))
  (`Controller.Possess` (`local.ControllerRef`) _returnvalue))

(fn `ChangeAnimState`
  (params (NewState :type "ECharAnimState Enum" :default "CAS_UNKNOWN"))
  (bind _naytiri_animation (`self.Naytiri_Animation`))
  (bind _naytiri_animation_2 (`self.Naytiri_Animation`))
  (bind _charactermovement (`self.CharacterMovement`))
  (`self.Naytiri_Animation`
    (:`then`
      (switch `ECharAnimState` NewState
        (:`CAS_IDLE`
          ;[1 1 1] Idle
          (`/Game/Final/Animations/Naytiri_AnimBP_BaseCharacter.ChangeAnimStateTime` (`self.Naytiri_Animation`) "CAS_IDLE" 0.0 null)
          (set `CharacterMovementComponent.RotationRate` (struct :`Yaw` 360.0) _charactermovement)
          (set `self.MovementScale` 1.0)
          (`parent.ChangeAnimState` (`local.NewState`) :!label _label))
        (:`CAS_ATTACK`
          ;[1 1 1] Attack
          (if (`|EnumEquality` (`self.AnimState`) "CAS_IDLE")
            (if (not (`self.SlowAttack`))
              (`/Game/Final/Animations/Naytiri_AnimBP_BaseCharacter.ChangeAnimStateTime` _naytiri_animation_2 "CAS_ATTACK" 1.0 "/Game/Final/Animations/Naytiri_SwordShield_Sword_Attack_3.Naytiri_SwordShield_Sword_Attack_3")
              (else
                (`/Game/Final/Animations/Naytiri_AnimBP_BaseCharacter.ChangeAnimStateTime` _naytiri_animation_2 "CAS_ATTACK" 1.0 "/Game/Final/Animations/Naytiri_SwordShield_Sword_Attack_1.Naytiri_SwordShield_Sword_Attack_1")))
            (set `CharacterMovementComponent.RotationRate` (struct :`Yaw` 60.0) _charactermovement)
            (set `self.MovementScale` 0.1)
            (goto _label)))
        (:`CAS_DAMAGE`
          (`/Game/Final/Animations/Naytiri_AnimBP_BaseCharacter.ChangeAnimStateTime` _naytiri_animation "CAS_DAMAGE" (`self.RecoveryDuration`) null)
          (goto _label))
        (:`CAS_DEATH`
          (`/Game/Final/Animations/Naytiri_AnimBP_BaseCharacter.ChangeAnimStateTime` _naytiri_animation "CAS_DEATH" 1.5 null)
          (goto _label))
        (:`CAS_CAST`
          (if (not (`self.MagicSlowAttack`))
            (`/Game/Final/Animations/Naytiri_AnimBP_BaseCharacter.ChangeAnimStateTime` _naytiri_animation "CAS_CAST" 2.5 "/Game/MagicalAnimSet/Animations/attack/02_shot/Naytiri_ShotC.Naytiri_ShotC")
            (else
              (`/Game/Final/Animations/Naytiri_AnimBP_BaseCharacter.ChangeAnimStateTime` _naytiri_animation "CAS_CAST" 2.5 "/Game/MagicalAnimSet/Animations/attack/10_buff/10_buff.10_buff")))
          (set `CharacterMovementComponent.RotationRate` (struct :`Yaw` 60.0) (`self.CharacterMovement`) :!label _label_2)
          (set `self.MovementScale` 0.1)
          (goto _label))
        (:`CAS_SPECIAL`
          (`/Game/Final/Animations/Naytiri_AnimBP_BaseCharacter.ChangeAnimStateTime` (`self.Naytiri_Animation`) "CAS_SPECIAL" 7.0 "/Game/MagicalAnimSet/Animations/attack/06_chanting/SpecialAttack.SpecialAttack")
          (goto _label_2))))
    (:`else`)))

(fn `CharacterDied`
  (`self.Ragdoll`)
  (`PrimitiveComponent.SetCollisionEnabled` (`self.CapsuleComponent`) "NoCollision")
  (set `SpringArmComponent.bDoCollisionTest` false (`self.mSpringArm`))
  (`self.DeathScreen`)
  (`SceneComponent.SetVisibility` (`self.PlayerName`) false false)
  (`SceneComponent.SetVisibility` (`self.Index`) false false))

(fn `ModifyDamage`
  (params (damage :type "Float (double-precision)"))
  (returns (ReturnValue :type "Float (double-precision)"))
  (`self.ChangeAnimStateMulti` "CAS_DAMAGE")
  (return damage))

(fn `onAttack`
  (for _array_element (`PrimitiveComponent.GetOverlappingActors` (`self.AttackRadius`) "/Game/Blueprints/Physics/BP_Hanging_Trap.BP_Hanging_Trap_C")
    ;[1 1 1] Trap
    (bind _asbp_hanging_trap (cast `/Game/Blueprints/Physics/BP_Hanging_Trap` _array_element))
    (bind _returnvalue (`self.GetDotProductTo` _asbp_hanging_trap))
    (`KismetSystemLibrary.PrintString` (`KismetStringLibrary.Conv_DoubleToString` _returnvalue))
    (if (> _returnvalue 0.1)
      (`/Game/Blueprints/Physics/BP_Hanging_Trap.BreakConstraint` _asbp_hanging_trap)))
  (for _array_element_2 (`PrimitiveComponent.GetOverlappingActors` (`self.AttackRadius`) "/Script/Engine.Actor")
    (if (> (`self.GetDotProductTo` _array_element_2) 0.3)
      (if (not (`self.SlowAttack`))
        (`GameplayStatics.ApplyDamage` _array_element_2 (`self.AttackDamage`))
        (`KismetSystemLibrary.PrintString` "Attack!")
        (else
          (`GameplayStatics.ApplyDamage` _array_element_2 (`self.AttackDamage`))
          (`KismetSystemLibrary.PrintString` "SlowAttack!"))))))

(fn `UserConstructionScript`)