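; BP_Enemy is a melee AI enemy character that chases and attacks the player.
; On BeginPlay it caches its AnimBP_BaseCharacter, then loops AIMoveTo toward the player, triggering a timed attack animation on arrival while the avatar lives and retrying after a short delay.
; OnAttack applies damage only when the player is in front, checked by dot product.
; Incoming damage and death switch animation state through an overridden ChangeAnimState.
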(event `self.ReceiveBeginPlay`
  (bind _asanim_bp_base_character (cast `/Game/Blueprints/AnimBP_BaseCharacter` (`SkeletalMeshComponent.GetAnimInstance` (`self.Mesh`))))
  (set `self.Animation` _asanim_bp_base_character)
  (`|AIMoveTo` self (0.0 0.0 0.0) (`GameplayStatics.GetPlayerPawn` 0) 100.0 :!label _label
    (:`OnSuccess`
      (bind _asbp_avatar (cast `/Game/Blueprints/BP_Avatar` (`GameplayStatics.GetPlayerPawn` 0)))
      (if (not (`COA_BaseCharacter.bDead` _asbp_avatar))
        (`self.ChangeAnimState` "CAS_ATTACK")
        (`KismetSystemLibrary.Delay` 1.5 :!label _label_2)
        (goto _label)))
    (:`OnFail`
      (goto _label_2))))

(event `self.CharacterDied`
  (`self.ChangeAnimState` "CAS_DEATH"))

(event `self.onAttack`
  (if (> (`self.GetDotProductTo` (`GameplayStatics.GetPlayerPawn` 0)) 0.3)
    (`GameplayStatics.ApplyDamage` (`GameplayStatics.GetPlayerPawn` 0) 20.0)))

(fn `ChangeAnimState`
  (params (NewState :type "ECharAnimState Enum" :default "CAS_UNKNOWN"))
  (`parent.ChangeAnimState` NewState)
  (bind _animation (`self.Animation`)
    (:`then`
      (`/Game/Blueprints/AnimBP_BaseCharacter.ChangeAnimStateTime` _animation NewState 1.0 "/Game/Mannequin/Animations/SwordShield_Sword_Attack_3.SwordShield_Sword_Attack_3"))
    (:`else`)))

(fn `ModifyDamage`
  (params (damage :type "Float (double-precision)"))
  (returns (ReturnValue :type "Float (double-precision)"))
  (`self.ChangeAnimState` "CAS_DAMAGE")
  (return damage))

(fn `UserConstructionScript`)