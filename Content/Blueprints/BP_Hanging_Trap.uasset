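; BP_Hanging_Trap is a physics trap hung on a cable and constraint that damages COA_BaseCharacter actors it hits.
; On begin play it sets the constraint's angular orientation target.
; BreakConstraint marks it cut, detaches the cable end, breaks the constraint and enables mesh physics simulation.
; Any hit damages while uncut, but only hard impacts do once cut, with damage scaled by clamped impulse magnitude.
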(event `self.ReceiveBeginPlay`
  (`PhysicsConstraintComponent.SetAngularOrientationTarget` (`self.PhysicsConstraint`) (`self.AngularDrive`)))

(event `self.ReceiveHit`
  (params (MyComp :type "PrimitiveComponent Object Reference") (Other :type "Actor Object Reference") (OtherComp :type "PrimitiveComponent Object Reference") (bSelfMoved :type Boolean) (HitLocation :type "Vector Structure") (HitNormal :type "Vector Structure") (NormalImpulse :type "Vector Structure") (Hit :type "HitResult Structure (by ref)"))
  (bind _returnvalue (`KismetMathLibrary.VSize` NormalImpulse))
  (bind _ascoa_base_character (cast `COA_BaseCharacter` Other))
  (if (or (> _returnvalue 16000.0) (not (`self.Cut?`)))
    (`KismetSystemLibrary.PrintString` (`KismetStringLibrary.Conv_DoubleToString` _returnvalue))
    (`GameplayStatics.ApplyDamage` _ascoa_base_character (`KismetMathLibrary.MapRangeClamped` _returnvalue 16000.0 50000.0 10.0 40.0) null self)))

(event `BreakConstraint`
  (set `self.Cut?` true)
  (set `CableComponent.bAttachEnd` false (`self.Cable`))
  (`PhysicsConstraintComponent.BreakConstraint` (`self.PhysicsConstraint`))
  (`PrimitiveComponent.SetSimulatePhysics` (`self.StaticMesh`) true))

(fn `UserConstructionScript`)