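; COA game mode that handles player numbering, start point selection and respawning.
; On login it stamps each BP_COAPlayerState with an incrementing PlayerIndex.
; ChoosePlayerStart spreads players across all PlayerStarts by wrapping their position in the GameState PlayerArray, independently of PlayerIndex.
; RespawnRequested spawns a new BP_Naytiri at the supplied transform and has the controller possess it after a short delay.
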(event `self.K2_PostLogin`
  (params (NewPlayer :type "PlayerController Object Reference"))
  (bind _lastplayerindex (`self.LastPlayerIndex`))
  (bind _asbp_coaplayer_state (cast `/Game/Blueprints/BP_COAPlayerState` (`Controller.PlayerState` NewPlayer)))
  (set `/Game/Blueprints/BP_COAPlayerState.PlayerIndex` _lastplayerindex _asbp_coaplayer_state)
  (`/Engine/EditorBlueprintResources/StandardMacros.IncrementInt` _lastplayerindex))

(event `RespawnRequested`
  (params (PlayerC :type "PlayerController Object Reference") (SpawnTransform :type "Transform Structure"))
  (`/Engine/EditorBlueprintResources/StandardMacros.IsValid` PlayerC
    (:`Is Valid`
      (bind _returnvalue (`|SpawnActorFromClass` "/Game/Blueprints/BP_Naytiri.BP_Naytiri_C" SpawnTransform "Undefined" "OverrideRootScale" null (struct) null))
      (`KismetSystemLibrary.Delay` 0.2)
      (`Controller.Possess` PlayerC _returnvalue))))

(fn `ChoosePlayerStart`
  (params (Player :type "Controller Object Reference"))
  (returns (ReturnValue :type "Actor Object Reference"))
  (bind _outactors (`GameplayStatics.GetAllActorsOfClass` "/Script/Engine.PlayerStart"))
  (return (`|GetArrayItem` _outactors (mod (`KismetArrayLibrary.Array_Find` (`GameStateBase.PlayerArray` (`GameplayStatics.GetGameState`)) (`Controller.PlayerState` Player)) (`KismetArrayLibrary.Array_Length` _outactors)))))

(fn `UserConstructionScript`)