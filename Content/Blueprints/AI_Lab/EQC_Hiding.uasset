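; EQS context for the hide-and-seek AI that supplies a set of character actors to environment queries.
; It gathers every BP_HideSeekChar, drops the querier's controlled pawn when the querier is a Controller, then removes characters flagged IsSeeker.
; Despite its SeekerList name, the returned array holds the other non-seeker characters.
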(fn `ProvideActorsSet`
  (params (QuerierObject :type "Object Object Reference") (QuerierActor :type "Actor Object Reference"))
  (returns (ResultingActorsSet :type "Array of Actor Object Reference"))
  (locals (AllCharacters :type "Array of /Game/Blueprints/AI_Lab/BP_HideSeekChar Object Reference") (SeekerList :type "Array of /Game/Blueprints/AI_Lab/BP_HideSeekChar Object Reference"))
  (bind _outactors (`GameplayStatics.GetAllActorsOfClass` "/Game/Blueprints/AI_Lab/BP_HideSeekChar.BP_HideSeekChar_C"))
  (bind _output_get (set `local.AllCharacters` _outactors))
  (set `local.SeekerList` _output_get)
  (bind _ascontroller (cast `Controller` QuerierActor)
    (:`then`
      (`KismetArrayLibrary.Array_RemoveItem` (`local.SeekerList`) (cast `/Game/Blueprints/AI_Lab/BP_HideSeekChar` (`Controller.K2_GetPawn` _ascontroller) :!pure true)))
    (:`CastFailed`
      _))
  (for _array_element (`local.AllCharacters`)
    (if (`/Game/Blueprints/AI_Lab/BP_HideSeekChar.IsSeeker?` _array_element)
      (`KismetArrayLibrary.Array_RemoveItem` (`local.SeekerList`) _array_element)))
  (return (`local.SeekerList`)))