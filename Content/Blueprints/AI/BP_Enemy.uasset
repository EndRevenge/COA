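; Enemy character Blueprint that deals melee damage to the player and reports death states to its AI Blackboard.
; OnAttack damages the player if roughly in front, then sets PlayerDead once their health runs out.
; ChangeAnimState drives the cached AnimBP for attack, damage and death, while CharacterDied disables capsule collision and sets IsDead.
; An older AIMoveTo chase-and-attack loop remains unconnected.
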(event `self.ReceiveBeginPlay`
  (bind _asanim_bp_base_character (cast `/Game/Blueprints/AnimBP_BaseCharacter` (`SkeletalMeshComponent.GetAnimInstance` (`self.Mesh`))))
  (set `self.Animation` _asanim_bp_base_character))

(event `self.ReceiveTick`
  (params (DeltaSeconds :type "Float (single-precision)")))

(event `self.CharacterDied`
  (bind _returnvalue (`AIBlueprintHelperLibrary.GetBlackboard` null))
  (`self.ChangeAnimState` "CAS_DEATH")
  (`PrimitiveComponent.SetCollisionEnabled` (`self.CapsuleComponent`) "NoCollision")
  ;[1 1 1] Stop Movement When Character Died
  (`/Engine/EditorBlueprintResources/StandardMacros.IsValid` _returnvalue
    (:`Is Valid`
      (`BlackboardComponent.SetValueAsBool` _returnvalue (`self.IsDead?`) true))))

(event `self.onAttack`
  (bind _returnvalue (`GameplayStatics.GetPlayerPawn` 0))
  (if (> (`self.GetDotProductTo` (`GameplayStatics.GetPlayerPawn` 0)) 0.3)
    (`GameplayStatics.ApplyDamage` _returnvalue 20.0)
    ;[1 1 1] Patrol After Player Dying
    (bind _asbp_avatar (cast `/Game/Blueprints/BP_Avatar` _returnvalue))
    (if (<= (`COA_BaseCharacter.Health` _asbp_avatar) 0.0)
      (`BlackboardComponent.SetValueAsBool` (`AIBlueprintHelperLibrary.GetBlackboard` null) (`self.PlayerDead`) true))))

(fn `ChangeAnimState`
  (params (NewState :type "ECharAnimState Enum" :default "CAS_UNKNOWN"))
  (`parent.ChangeAnimState` NewState)
  (bind _animation (`self.Animation`)
    (:`then`
      (`/Game/Blueprints/AnimBP_BaseCharacter.ChangeAnimStateTime` _animation NewState 1.0 "/Game/Mannequin/Animations/SwordShield_Sword_Attack_3.SwordShield_Sword_Attack_3"))
    (:`else`)))

(fn `ModifyDamage`
  (params (damage :type "Float (double-precision)"))
  (returns (ReturnValue :type "Float (double-precision)"))
  (`self.ChangeAnimState` "CAS_DAMAGE")
  (return damage))

(fn `UpdateWalkSpeed`
  (params (NewWalkSpeed :type "Float (double-precision)"))
  (set `CharacterMovementComponent.MaxWalkSpeed` NewWalkSpeed (`self.CharacterMovement`)))

(fn `UserConstructionScript`)