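; EQS context for the seeker AI in hide-and-seek, whose ProvideActorsSet override is empty as wired.
; An unconnected node chain gathers every BP_HideSeekChar, removes the querier controller's own pawn and any seekers, and returns the rest.
; That chain never runs, so the context provides no actors, and it also removes entries from the array it is looping over.
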(fn `ProvideActorsSet`
  (params (QuerierObject :type "Object Object Reference") (QuerierActor :type "Actor Object Reference"))
  (returns (ResultingActorsSet :type "Array of Actor Object Reference")))