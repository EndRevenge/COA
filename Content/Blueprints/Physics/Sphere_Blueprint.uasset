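; Sphere actor Blueprint that reports overlaps and impact strength through on-screen debug prints, apparently as a placeholder for impact sounds.
; Begin overlap prints the other actor's name.
; Hit sorts the negated X component of the normal impulse into three rising bands, each printing a Turkish "make sound" style message; no audio plays.
; A print of the raw impulse value is left unconnected.
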(event `self.ReceiveActorBeginOverlap`
  (params (OtherActor :type "Actor Object Reference"))
  (`KismetSystemLibrary.PrintString` (`KismetStringLibrary.Concat_StrStr` "Sphere overlapped with" (`KismetSystemLibrary.GetDisplayName` OtherActor))))

(event `self.ReceiveHit`
  (params (MyComp :type "PrimitiveComponent Object Reference") (Other :type "Actor Object Reference") (OtherComp :type "PrimitiveComponent Object Reference") (bSelfMoved :type Boolean) (HitLocation :type "Vector Structure") (HitNormal :type "Vector Structure") (NormalImpulse :type "Vector Structure") (Hit :type "HitResult Structure (by ref)"))
  (bind _returnvalue (* -1 (.x NormalImpulse)))
  (if (`KismetMathLibrary.InRange_FloatFloat` _returnvalue 0.6 1.0)
    (`KismetSystemLibrary.PrintString` "Ses Çıkar")
    (elif (`KismetMathLibrary.InRange_FloatFloat` _returnvalue 1.01 5.0)
      (`KismetSystemLibrary.PrintString` "Büyük Ses Çıkar")
      (elif (> _returnvalue 5.1)
        (`KismetSystemLibrary.PrintString` "En büyük Ses")))))

(fn `UserConstructionScript`)