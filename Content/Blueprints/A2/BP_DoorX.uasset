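; BP_DoorX is a swinging door that opens automatically when the BP_Naytiri character enters its box trigger.
; A dot product against that character picks the swing direction, positive or negative 90 degrees.
; The DoorOpening timeline drives the door mesh's yaw from the rotation stored at construction.
; Ending the overlap clears the Active guard and reverses the timeline after a one-second delay.
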(event `self.Box.OnComponentBeginOverlap`
  (params (OverlappedComponent :type "PrimitiveComponent Object Reference") (OtherActor :type "Actor Object Reference") (OtherComp :type "PrimitiveComponent Object Reference") (OtherBodyIndex :type Integer) (bFromSweep :type Boolean) (SweepResult :type "HitResult Structure (by ref)"))
  (bind (_startrot_roll _startrot_pitch _startrot_yaw) (`KismetMathLibrary.BreakRotator` (`self.StartRot`)))
  (if (not (`self.Active?`))
    (set `self.Active?` true)
    (bind _asbp_naytiri (cast `/Game/Blueprints/BP_Naytiri` OtherActor))
    (if (> (`self.GetDotProductTo` _asbp_naytiri) 0.55)
      (set `self.DotProduct` -90.0)
      (bind (_direction _doormoves) (`Timeline|DoorOpening` :!via `PlayFromStart` :!label _label)
        (:`Update`
          (`SceneComponent.K2_SetWorldRotation` (`self.Door`) (`KismetMathLibrary.MakeRotator` _startrot_roll _startrot_pitch (+ _startrot_yaw (* (`self.DotProduct`) (`KismetMathLibrary.FClamp` _doormoves 0.0 1.0)))) false false)))
      (else
        (set `self.DotProduct` 90.0)
        (goto _label :!via `PlayFromStart`)))))

(event `self.Box.OnComponentEndOverlap`
  (params (OverlappedComponent :type "PrimitiveComponent Object Reference") (OtherActor :type "Actor Object Reference") (OtherComp :type "PrimitiveComponent Object Reference") (OtherBodyIndex :type Integer))
  (set `self.Active?` false)
  (`KismetSystemLibrary.Delay` 1.0)
  (goto _label :!via `Reverse`))

(fn `UserConstructionScript`
  (set `self.StartRot` (`SceneComponent.K2_GetComponentRotation` (`self.Door`))))