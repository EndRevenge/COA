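; ChooseColor is an overlap-triggered actor that sets the costume color of a BP_Naytiri character that touches it.
; It writes its Color variable into the game instance's player settings, keeping display name and weapon type, then passes those settings to the character's SendPlayerSettingsServer.
; It also prints the color and applies it directly to the mesh's BodyColor material parameter.
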(event `self.ReceiveActorBeginOverlap`
  (params (OtherActor :type "Actor Object Reference"))
  (bind _asbp_avatar (cast `/Game/Blueprints/BP_Naytiri` OtherActor))
  (bind _asbp_coagame_instance (cast `/Game/Blueprints/BP_COAGameInstance` (`GameplayStatics.GetGameInstance`)))
  (bind (_settings_displayname _settings_costumecolor _settings_weapontype) (break `/Game/Blueprints/S_PlayerSettings` (`/Game/Blueprints/BP_COAGameInstance.Settings` _asbp_coagame_instance)))
  (bind _output_get (set `/Game/Blueprints/BP_COAGameInstance.Settings` (make `/Game/Blueprints/S_PlayerSettings` _settings_displayname (`self.Color`) _settings_weapontype) _asbp_coagame_instance))
  (`/Game/Blueprints/BP_Naytiri.SendPlayerSettingsServer` _asbp_avatar (make `/Game/Blueprints/S_PlayerSettings` (break `/Game/Blueprints/S_PlayerSettings` _output_get) (`.CostumeColor_7_84FAA5774FDCEC076465FD94E5A9119D` (break `/Game/Blueprints/S_PlayerSettings` _output_get)) (`.WeaponType_9_909028214361E467878D2E935A1A49CC` (break `/Game/Blueprints/S_PlayerSettings` _output_get))))
  (`KismetSystemLibrary.PrintString` (`KismetStringLibrary.Conv_ColorToString` (`.CostumeColor_7_84FAA5774FDCEC076465FD94E5A9119D` (break `/Game/Blueprints/S_PlayerSettings` _output_get))))
  (`MeshComponent.SetVectorParameterValueOnMaterials` (`Character.Mesh` _asbp_avatar) "BodyColor" (`KismetMathLibrary.Conv_LinearColorToVector` (`self.Color`))))

(fn `UserConstructionScript`)