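; ChooseWeapon is a pickup-style actor that sets the weapon type of a BP_Naytiri player that overlaps it.
; On overlap it writes its WeaponType into the game instance's player settings, keeping name and costume color, then sends those settings to the server.
; It also updates the character's Index text and calls ChangeWeapon.
; The construction script labels the actor's text render to match the configured weapon type.
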(event `self.ReceiveActorBeginOverlap`
  (params (OtherActor :type "Actor Object Reference"))
  (bind _asbp_naytiri (cast `/Game/Blueprints/BP_Naytiri` OtherActor))
  (bind _asbp_coagame_instance (cast `/Game/Blueprints/BP_COAGameInstance` (`GameplayStatics.GetGameInstance`)))
  (bind (_settings_displayname _settings_costumecolor) (break `/Game/Blueprints/S_PlayerSettings` (`/Game/Blueprints/BP_COAGameInstance.Settings` _asbp_coagame_instance)))
  (bind _output_get (set `/Game/Blueprints/BP_COAGameInstance.Settings` (make `/Game/Blueprints/S_PlayerSettings` _settings_displayname _settings_costumecolor (`self.WeaponType?`)) _asbp_coagame_instance))
  (`/Game/Blueprints/BP_Naytiri.SendPlayerSettingsServer` _asbp_naytiri (make `/Game/Blueprints/S_PlayerSettings` (break `/Game/Blueprints/S_PlayerSettings` _output_get) (`.CostumeColor_7_84FAA5774FDCEC076465FD94E5A9119D` (break `/Game/Blueprints/S_PlayerSettings` _output_get)) (`.WeaponType_9_909028214361E467878D2E935A1A49CC` (break `/Game/Blueprints/S_PlayerSettings` _output_get))))
  (`TextRenderComponent.K2_SetText` (`/Game/Blueprints/BP_Naytiri.Index` _asbp_naytiri) (`KismetTextLibrary.Conv_StringToText` (`|GetEnumeratorNameAsString` (`.WeaponType_9_909028214361E467878D2E935A1A49CC` (break `/Game/Blueprints/S_PlayerSettings` _output_get)))))
  (`/Game/Blueprints/BP_Naytiri.ChangeWeapon` _asbp_naytiri (`.WeaponType_9_909028214361E467878D2E935A1A49CC` (break `/Game/Blueprints/S_PlayerSettings` _output_get))))

(fn `UserConstructionScript`
  (switch `/Game/Blueprints/E_WeaponType` (`self.WeaponType?`)
    (:`NewEnumerator0`
      (`TextRenderComponent.K2_SetText` (`self.TextRender`) (`self.Text - Unarmed`)))
    (:`NewEnumerator1`
      (`TextRenderComponent.K2_SetText` (`self.TextRender`) (`self.Text - Sword`)))
    (:`NewEnumerator2`
      (`TextRenderComponent.K2_SetText` (`self.TextRender`) (`self.Text - Magic`)))))