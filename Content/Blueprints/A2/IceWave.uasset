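; IceWave is a short-lived attack actor that sends Ball1 along a spline and damages BP_Naytiri characters.
; Shortly after BeginPlay, the MovingWave timeline drives Ball1's local position and rotation along the spline, and the actor destroys itself seconds later.
; Sphere overlaps with BP_Naytiri apply radial damage around the actor's origin, sparing WhoCast and passing the overlapped character as damage causer.
; An attach-to-caster call is left unconnected.
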(event `self.ReceiveBeginPlay`
  (`KismetSystemLibrary.Delay` 0.2)
  (`self.MoveDarling`)
  (`KismetSystemLibrary.Delay` 3.0)
  (`self.K2_DestroyActor`))

(event `MoveDarling`
  (bind _spline (`self.Spline`))
  (bind (_direction _spherical) (`Timeline|MovingWave` :!via `PlayFromStart`)
    (:`Update`
      (bind _returnvalue (`KismetMathLibrary.Lerp` 0.0 (`SplineComponent.GetSplineLength` _spline) _spherical))
      (`SceneComponent.K2_SetRelativeLocationAndRotation` (`self.Ball1`) (`SplineComponent.GetLocationAtDistanceAlongSpline` _spline _returnvalue "Local") (`SplineComponent.GetRotationAtDistanceAlongSpline` _spline _returnvalue "Local") false false))))

(event `self.Sphere.OnComponentBeginOverlap`
  (params (OverlappedComponent :type "PrimitiveComponent Object Reference") (OtherActor :type "Actor Object Reference") (OtherComp :type "PrimitiveComponent Object Reference") (OtherBodyIndex :type Integer) (bFromSweep :type Boolean) (SweepResult :type "HitResult Structure (by ref)"))
  (bind _asbp_naytiri (cast `/Game/Blueprints/BP_Naytiri` OtherActor))
  (`GameplayStatics.ApplyRadialDamage` 60.0 (`self.K2_GetActorLocation`) (`SphereComponent.SphereRadius` (`self.Sphere`)) null (`|MakeArray` (`self.WhoCast?`) :!type "Actor Object Reference") _asbp_naytiri null))

(fn `UserConstructionScript`)