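; BP_Lever is a lever that tilts while BP_Naytiri overlaps its box.
; On overlap, a timeline plays from start, adding up to 30 degrees of pitch to the lever's rotation captured in the construction script.
; Any overlap sets the Active guard before the character cast, and any end overlap clears it, then reverses the timeline after a short delay.
; The stored world rotation is applied as relative rotation.
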(event `self.Box.OnComponentBeginOverlap`
  (params (OverlappedComponent :type "PrimitiveComponent Object Reference") (OtherActor :type "Actor Object Reference") (OtherComp :type "PrimitiveComponent Object Reference") (OtherBodyIndex :type Integer) (bFromSweep :type Boolean) (SweepResult :type "HitResult Structure (by ref)"))
  (bind (_startrot_roll _startrot_pitch _startrot_yaw) (`KismetMathLibrary.BreakRotator` (`self.StartRot`)))
  (if (not (`self.Active?`))
    (set `self.Active?` true)
    (cast `/Game/Blueprints/BP_Naytiri` OtherActor)
    (bind (_direction _levermoves) (`Timeline|LeverM` :!via `PlayFromStart` :!label _label)
      (:`Update`
        (`SceneComponent.K2_SetRelativeRotation` (`self.Lever`) (`KismetMathLibrary.MakeRotator` _startrot_roll (+ _startrot_pitch (* 30.0 (`KismetMathLibrary.FClamp` _levermoves))) _startrot_yaw) false false)))))

(event `self.Box.OnComponentEndOverlap`
  (params (OverlappedComponent :type "PrimitiveComponent Object Reference") (OtherActor :type "Actor Object Reference") (OtherComp :type "PrimitiveComponent Object Reference") (OtherBodyIndex :type Integer))
  (set `self.Active?` false)
  (`KismetSystemLibrary.Delay` 1.0)
  (goto _label :!via `Reverse`))

(fn `UserConstructionScript`
  (set `self.StartRot` (`SceneComponent.K2_GetComponentRotation` (`self.Lever`))))