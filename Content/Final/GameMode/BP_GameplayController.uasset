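; BP_GameplayController is a player controller that toggles the main menu widget as a pause menu during gameplay.
; The Pause input and the PauseMenu event share one path that lazily creates MainMenu_W, caches it, then adds or removes it from the viewport.
; Showing it enables the cursor and UI-only input, and hiding it restores game-only input.
; It never pauses the game itself.
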(event `PauseMenu`
  ;[1 0.6282 0] Pause - Create widget - Add to viewport - UI only
  (`/Engine/EditorBlueprintResources/StandardMacros.IsValid` (`self.MainMenu_W`) :!label _label
    (:`Is Valid`
      (if (`Widget.IsInViewport` (`self.MainMenu_W`))
        (`Widget.RemoveFromParent` (`self.MainMenu_W`))
        (set `self.bShowMouseCursor` false)
        (`WidgetBlueprintLibrary.SetInputMode_GameOnly` self)
        (else
          (`UserWidget.AddToViewport` (stale _output_get) 0 :!label _label_2)
          (set `self.bShowMouseCursor` true)
          (`WidgetBlueprintLibrary.SetInputMode_UIOnlyEx` self null))))
    (:`Is Not Valid`
      (bind _returnvalue (`|CreateWidget` "/Game/Final/Widget/MainMenu_W.MainMenu_W_C"))
      (bind _output_get (set `self.MainMenu_W` _returnvalue))
      (goto _label_2))))

(event `InputAction|Pause`
  (params (Key :type "Key Structure"))
  ;[1 0.6282 0] Pause - Create widget - Add to viewport - UI only
  (:`Pressed`
    (goto _label)))

(fn `UserConstructionScript`)