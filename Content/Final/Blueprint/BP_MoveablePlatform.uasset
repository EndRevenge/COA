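; BP_MoveablePlatform is a platform that moves along a configurable offset and can carry a bear and a blade actor.
; On BeginPlay it attaches both actors to its mesh, keeping world transforms, but only if both references are valid.
; The MovePlatform timeline, rate-scaled by Seconds, drives the mesh's relative location as a fraction of the Movement vector.
; The construction script scales the mesh, using Length for the Y axis.
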(event `self.ReceiveBeginPlay`
  (bind _staticmesh (`self.StaticMesh`))
  (`|ExecutionSequence`
    (:`then_0`
      (bind _bp_blade (`self.BP_Blade`)
        (:`then`
          (bind _bp_bear (`self.BP_Bear`)
            (:`then`
              (`SceneComponent.K2_AttachToComponent` (`Actor.RootComponent` _bp_bear) _staticmesh "None" "KeepWorld" "KeepWorld" "KeepWorld" true)
              (`SceneComponent.K2_AttachToComponent` (`Actor.RootComponent` _bp_blade) _staticmesh "None" "KeepWorld" "KeepWorld" "KeepWorld" true))
            (:`else`)))
        (:`else`)))
    (:`then_1`
      (`TimelineComponent.SetPlayRate` (`self.MovePlatform`) (/ 2.0 (`self.Seconds`)))
      (bind (_direction _movementamount) (`Timeline|MovePlatform` :!via `PlayFromStart`)
        (:`Update`
          (`SceneComponent.K2_SetRelativeLocation` (`self.StaticMesh`) (* (`self.Movement`) _movementamount) false false))))))

(fn `UserConstructionScript`
  (`SceneComponent.SetRelativeScale3D` (`self.StaticMesh`) (`KismetMathLibrary.MakeVector` (`self.New Scale 3D X`) (`self.Length`) (`self.New Scale 3D Z`))))