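; BP_TutorialSpawn is a trigger volume that shows a tutorial popup when the local player's BP_Naytiri enters it.
; On first overlap it halts the character's movement, creates a Tutorial_W with the configured TextDescription, and switches to Game-and-UI input with the cursor visible.
; The Continue input, or the actor's destruction, calls the widget's Continue and plays a whip sound.
; The construction script sizes the box from BoxExtent.
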(event `self.ReceiveBeginPlay`)

(event `self.Box.OnComponentBeginOverlap`
  (params (OverlappedComponent :type "PrimitiveComponent Object Reference") (OtherActor :type "Actor Object Reference") (OtherComp :type "PrimitiveComponent Object Reference") (OtherBodyIndex :type Integer) (bFromSweep :type Boolean) (SweepResult :type "HitResult Structure (by ref)"))
  (bind _returnvalue (`self.GetInstigatorController` OtherActor))
  (`/Engine/EditorBlueprintResources/StandardMacros.IsValid` _returnvalue
    (:`Is Valid`
      (if (`Controller.IsLocalPlayerController` _returnvalue)
        (bind _asbp_naytiri (cast `/Game/Blueprints/BP_Naytiri` OtherActor))
        (`MovementComponent.StopMovementImmediately` (`Character.CharacterMovement` _asbp_naytiri))
        (bind _asbp_gameplay_controller (cast `/Game/Final/GameMode/BP_GameplayController` _returnvalue)
          (:`then`
            (`/Engine/EditorBlueprintResources/StandardMacros.DoOnce` false
              (:`Completed`
                (`/Engine/EditorBlueprintResources/StandardMacros.IsValid` (`self.Tutorial_W`)
                  (:`Is Valid`
                    _)
                  (:`Is Not Valid`
                    (bind _returnvalue_2 (`|CreateWidget` "/Game/Final/Widget/Tutorial_W.Tutorial_W_C" _asbp_gameplay_controller (`self.Text Description`)))
                    (bind _output_get (set `self.Tutorial_W` _returnvalue_2))))
                (`UserWidget.AddToViewport` _output_get 0)
                (`WidgetBlueprintLibrary.SetInputMode_GameAndUIEx` (`GameplayStatics.GetPlayerController` 0) _output_get "DoNotLock" false)
                (set `PlayerController.bShowMouseCursor` true (`GameplayStatics.GetPlayerController` 0)))))
          (:`CastFailed`
            (`KismetSystemLibrary.PrintString` "BP_TutorialSpawn cast failed." true true (struct :`R` 1.0 :`B` 0.040784 :`A` 1.0) 5.0)))))))

(event `self.ReceiveDestroyed`
  (`/Game/Final/Widget/Tutorial_W.Continue` (`self.Tutorial_W`) :!label _label)
  (`GameplayStatics.PlaySound2D` "/Game/Final/Audio/Whip.Whip" 1.0 1.0 0.0 null null))

(event `InputAction|Continue`
  (params (Key :type "Key Structure"))
  (:`Pressed`
    (goto _label)))

(fn `UserConstructionScript`
  (`BoxComponent.SetBoxExtent` (`self.Box`) (`self.Box Extent`) true))