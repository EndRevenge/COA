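; BP_WinOrLoseSpawn is a trigger volume, sized by BoxExtent in construction, that starts the win check between BP_Naytiri characters.
; An overlapping BP_Naytiri has its death-screen and win flags cleared and starts a one-second looping poll of all BP_Naytiri actors.
; When one is dead, the poll calls WinOrLoseScreen(true) on those still alive and clears its timer.
; An older widget-spawning path is left disconnected.
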(event `self.ReceiveBeginPlay`)

(event `self.Box.OnComponentBeginOverlap`
  (params (OverlappedComponent :type "PrimitiveComponent Object Reference") (OtherActor :type "Actor Object Reference") (OtherComp :type "PrimitiveComponent Object Reference") (OtherBodyIndex :type Integer) (bFromSweep :type Boolean) (SweepResult :type "HitResult Structure (by ref)"))
  (bind _output_get (set `self.Other Actor` OtherActor))
  (`/Engine/EditorBlueprintResources/StandardMacros.IsValid` _output_get
    (:`Is Valid`
      (bind _asbp_naytiri (cast `/Game/Blueprints/BP_Naytiri` OtherActor)
        (:`then`
          (set `/Game/Blueprints/BP_Naytiri.SpawnDeathScreen?` false _asbp_naytiri)
          (set `/Game/Blueprints/BP_Naytiri.Win?` false _asbp_naytiri)
          (`KismetSystemLibrary.PrintString` "WIN OR LOSE BP" true true (struct :`G` 0.66 :`B` 1.0 :`A` 1.0) 5.0)
          (`KismetSystemLibrary.K2_SetTimer` null "GetAllActors" 1.0 true))
        (:`CastFailed`
          (`KismetSystemLibrary.PrintString` "cast failed"))))))

(event `GetAllActors`
  (bind _outactors (`GameplayStatics.GetAllActorsOfClass` "/Game/Blueprints/BP_Naytiri.BP_Naytiri_C"))
  (for _array_element _outactors
    (if (`COA_BaseCharacter.bDead` _array_element)
      (`KismetSystemLibrary.PrintString` "BiriÖldü")
      (`self.NotDeadGuy`)
      (`KismetSystemLibrary.K2_ClearTimer` null "GetAllActors"))))

(event `NotDeadGuy`
  (bind _outactors (`GameplayStatics.GetAllActorsOfClass` "/Game/Blueprints/BP_Naytiri.BP_Naytiri_C"))
  (for _array_element _outactors
    (if (not (`COA_BaseCharacter.bDead` _array_element))
      (`/Game/Blueprints/BP_Naytiri.WinOrLoseScreen` _array_element true)
      (`KismetSystemLibrary.PrintString` "AAAAAAAAAAAA" true true (struct :`G` 1.0 :`B` 0.158461 :`A` 1.0)))))

(event `self.ReceiveTick`
  (params (DeltaSeconds :type "Float (single-precision)")))

(fn `UserConstructionScript`
  (`BoxComponent.SetBoxExtent` (`self.Box`) (`self.Box Extent`) true))